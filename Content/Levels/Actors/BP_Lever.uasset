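; BP_Lever is a level lever that switches a linked puzzle actor on and off when interacted with.
; It starts with the off sprite, and each Interact swaps the sprite based on IsOn, then calls Activate or DeActivate on PuzzleActor.
; IsOn only flips when PuzzleActor is valid, so an unlinked lever shows the on sprite after interaction and never switches back.
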(event EventBeginPlay
  ;[1 1 1] Set sprite
  (Rendering|Components|Sprite|SetSprite (Variables|Default|GetLever) (Variables|Default|GetLeverOff)))

(event EventInteract
  (bind _puzzleactor (Variables|Default|GetPuzzleActor))
  (bind _puzzleactor_2 (Variables|Default|GetPuzzleActor))
  ;[1 1 1] Call interact on puzzle actor blueprints
  (if (Variables|Default|GetIsOn?)
    (Rendering|Components|Sprite|SetSprite (Variables|Default|GetLever) (Variables|Default|GetLeverOff))
    (Utilities|IsValid _puzzleactor
      (:Is%20Valid
        (Class|PuzzleActor|DeActivate _puzzleactor)
        (Variables|Default|SetIsOn? false)))
    (else
      (Rendering|Components|Sprite|SetSprite (Variables|Default|GetLever) (Variables|Default|GetLeverOn))
      (Utilities|IsValid _puzzleactor_2
        (:Is%20Valid
          (Class|PuzzleActor|Activate _puzzleactor_2)
          (Variables|Default|SetIsOn? true))))))

(fn ConstructionScript)