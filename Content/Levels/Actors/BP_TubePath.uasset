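; Tube actor that carries a BP_Circle along a spline between its entrance and exit boxes, in either direction.
; Overlapping the entrance plays the MovementDuration timeline forward and the exit plays it in reverse, at a rate of TimelineSpeed over TimelineDuration.
; During travel the circle is rescaled with collision off and InputDisabled set, which also blocks retriggering.
; When the timeline finishes, it restores input, unit scale and collision.
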(event OnComponentBeginOverlap(EntranceBox)
  (params (OverlappedComponent :type Primitive%20Component%20Object%20Reference) (OtherActor :type Actor%20Object%20Reference) (OtherComp :type Primitive%20Component%20Object%20Reference) (OtherBodyIndex :type Integer) (bFromSweep :type Boolean) (SweepResult :type Hit%20Result%20Structure%20%28by%20ref%29))
  ;[1 1 1] Box Overlaps
  (bind _asbp_circle (Utilities|Casting|CastToBP_Circle OtherActor))
  (bind _output_get (Variables|Default|SetBP_CircleRef _asbp_circle))
  (if (not (Variables|/Script/shape_science_jam.Shape|GetInputDisabled _output_get))
    (Variables|Default|SetMoveInReverse false)
    (CallFunction|MoveCircle)))

(event OnComponentBeginOverlap(ExitBox)
  (params (OverlappedComponent :type Primitive%20Component%20Object%20Reference) (OtherActor :type Actor%20Object%20Reference) (OtherComp :type Primitive%20Component%20Object%20Reference) (OtherBodyIndex :type Integer) (bFromSweep :type Boolean) (SweepResult :type Hit%20Result%20Structure%20%28by%20ref%29))
  ;[1 1 1] Box Overlaps
  (bind _asbp_circle (Utilities|Casting|CastToBP_Circle OtherActor))
  (bind _output_get (Variables|Default|SetBP_CircleRef _asbp_circle))
  (if (not (Variables|/Script/shape_science_jam.Shape|GetInputDisabled _output_get))
    (Variables|Default|SetMoveInReverse true)
    (CallFunction|MoveCircle)))

(event Custom|MoveCircle
  (bind _bp_circleref (Variables|Default|GetBP_CircleRef))
  (bind _path (Variables|Default|GetPath))
  ;[1 1 1] Path movement
  (Utilities|IsValid _bp_circleref
    (:Is%20Valid
      (Transformation|SetActorScale3D _bp_circleref (Variables|Default|GetShapeScale3d))
      (Collision|SetActorEnableCollision (Variables|Default|GetBP_CircleRef) false)
      (Variables|/Script/shape_science_jam.Shape|SetInputDisabled (Variables|Default|GetBP_CircleRef) true)
      (Components|Timeline|SetPlayRate (Variables|Default|GetMovementDuration) (/ (Variables|Default|GetTimelineSpeed) (Variables|Default|GetTimelineDuration)))
      (if (not (Variables|Default|GetMoveInReverse))
        (bind _splinemovement (Timeline|MovementDuration PlayFromStart)
          (:Update
            (Transformation|SetActorLocationAndRotation (Variables|Default|GetBP_CircleRef) (Spline|GetLocationatDistanceAlongSpline _path (Math|Float|Lerp 0.0 _splinemovement (Spline|GetSplineLength _path)) "World")))
          (:Finished
            (Variables|/Script/shape_science_jam.Shape|SetInputDisabled (Variables|Default|GetBP_CircleRef) false)
            (Transformation|SetActorScale3D (Variables|Default|GetBP_CircleRef) "1.000000,1.000000,1.000000")
            (Collision|SetActorEnableCollision (Variables|Default|GetBP_CircleRef) true)))
        (else
          (Timeline|MovementDuration ReverseFromEnd))))))

(fn ConstructionScript)