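; BP_Door is a sliding door actor that moves between its starting position and an offset open position when Open or Close is called.
; BeginPlay derives the end location from the sprite and TransformDistance, though the final branch repeats the Door_Vertical check and is unreachable.
; DoorTransformTimeline plays or reverses, feeding its track as DeltaTime into VInterpTo to set the location.
; KillZone overlap only casts to Shape, with no further action.
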(event OnComponentBeginOverlap(KillZone)
  (params (OverlappedComponent :type Primitive%20Component%20Object%20Reference) (OtherActor :type Actor%20Object%20Reference) (OtherComp :type Primitive%20Component%20Object%20Reference) (OtherBodyIndex :type Integer) (bFromSweep :type Boolean) (SweepResult :type Hit%20Result%20Structure%20%28by%20ref%29))
  (Utilities|Casting|CastToShape OtherActor))

(event Custom|Open
  ;[1 1 1] Open/Close Door
  (bind _transform (Timeline|Door%20Transform%20Timeline Play)
    (:Update
      (Transformation|SetActorLocation (Math|Interpolation|VInterpTo (Variables|Default|GetStarting%20Location) (Variables|Default|GetEnding%20Location) _transform (Variables|Default|GetTransformSpeed)) false false))))

(event Custom|Close
  ;[1 1 1] Open/Close Door
  (bind _transform (Timeline|Door%20Transform%20Timeline Reverse)
    (:Update
      (Transformation|SetActorLocation (Math|Interpolation|VInterpTo (Variables|Default|GetStarting%20Location) (Variables|Default|GetEnding%20Location) _transform (Variables|Default|GetTransformSpeed)) false false))))

(event EventBeginPlay
  ;[1 1 1] Get Door Default Position
  (Variables|Default|SetStarting%20Location (Transformation|GetActorLocation))
  (if (== (Sprite|GetSprite (Variables|Default|GetDoor%20Sprite)) "/Game/Import_Assets/Sprites/Buttons/Door_Vertical.Door_Vertical")
    (Variables|Default|SetEnding%20Location (Math|Vector|MakeVector (.x (Variables|Default|GetStarting%20Location)) (.y (Variables|Default|GetStarting%20Location)) (+ (.z (Variables|Default|GetStarting%20Location)) (Variables|Default|GetTransformDistance))))
    (elif (== (Sprite|GetSprite (Variables|Default|GetDoor%20Sprite)) "/Game/Import_Assets/Sprites/Buttons/Door_Vertical_1.Door_Vertical_1")
      (Variables|Default|SetEnding%20Location (Math|Vector|MakeVector (.x (Variables|Default|GetStarting%20Location)) (.y (Variables|Default|GetStarting%20Location)) (- (.z (Variables|Default|GetStarting%20Location)) (Variables|Default|GetTransformDistance))))
      (elif (== (Sprite|GetSprite (Variables|Default|GetDoor%20Sprite)) "/Game/Import_Assets/Sprites/Buttons/Door_Horizontal.Door_Horizontal")
        (Variables|Default|SetEnding%20Location (Math|Vector|MakeVector (- (.x (Variables|Default|GetStarting%20Location)) (Variables|Default|GetTransformDistance)) (.y (Variables|Default|GetStarting%20Location)) (.z (Variables|Default|GetStarting%20Location))))
        (elif (== (Sprite|GetSprite (Variables|Default|GetDoor%20Sprite)) "/Game/Import_Assets/Sprites/Buttons/Door_Vertical.Door_Vertical")
          (Variables|Default|SetEnding%20Location (Math|Vector|MakeVector (+ (.x (Variables|Default|GetStarting%20Location)) (Variables|Default|GetTransformDistance)) (.y (Variables|Default|GetStarting%20Location)) (.z (Variables|Default|GetStarting%20Location)))))))))

(fn ConstructionScript)