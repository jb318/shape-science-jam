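; BP_Glass is a level actor that carries an overlapping Circle along a spline path.
; Entering EntranceBox stores the Circle and starts MoveCircle, which disables its input, applies a configured scale and drives it with a timeline at adjustable speed.
; Timeline progress maps to distance along the spline, and finishing restores input and unit scale.
; A reverse-playback branch exists, but the entrance overlap always selects forward playback despite setting MoveInReverse to true.
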(event OnComponentBeginOverlap(EntranceBox)
  (params (OverlappedComponent :type Primitive%20Component%20Object%20Reference) (OtherActor :type Actor%20Object%20Reference) (OtherComp :type Primitive%20Component%20Object%20Reference) (OtherBodyIndex :type Integer) (bFromSweep :type Boolean) (SweepResult :type Hit%20Result%20Structure%20%28by%20ref%29))
  ;[1 1 1] Box Overlaps
  (bind _ascircle (Utilities|Casting|CastToCircle OtherActor))
  (Variables|Default|SetCircle_Ref _ascircle)
  (Variables|Default|Set!MoveInReverse true)
  (Variables|Default|SetEntered%20A%20to%20B true)
  (CallFunction|MoveCircle))

(event Custom|MoveCircle
  (bind _circle_ref (Variables|Default|GetCircle_Ref))
  (bind _path (Variables|Default|GetPath))
  ;[1 1 1] Path movement
  (Utilities|IsValid _circle_ref
    (:Is%20Valid
      (Transformation|SetActorScale3D _circle_ref (Variables|Default|GetShapeScale3d))
      (Variables|/Script/shape_science_jam.Shape|SetInputDisabled (Variables|Default|GetCircle_Ref) true)
      (Components|Timeline|SetPlayRate (Variables|Default|GetMovementDuration) (/ (Variables|Default|GetTimelineSpeed) (Variables|Default|GetTimelineDuration)))
      (if (Variables|Default|Get!MoveInReverse)
        (bind _splinemovement (Timeline|MovementDuration Play)
          (:Update
            (Transformation|SetActorLocationAndRotation (Variables|Default|GetCircle_Ref) (Spline|GetLocationatDistanceAlongSpline _path (Math|Float|Lerp 0.0 _splinemovement (Spline|GetSplineLength _path)) "World")))
          (:Finished
            (Variables|/Script/shape_science_jam.Shape|SetInputDisabled (Variables|Default|GetCircle_Ref) false)
            (Transformation|SetActorScale3D (Variables|Default|GetCircle_Ref) "1.000000,1.000000,1.000000")))
        (else
          (Timeline|MovementDuration ReverseFromEnd))))))

(fn ConstructionScript)