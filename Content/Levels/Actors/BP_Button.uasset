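; BP_Button is a level pressure button that opens a linked door while a Shape actor overlaps it.
; Overlap begin and end swap the button sprite, play a sound, switch the linked light and open or close the door.
; Paired DoOnce nodes re-arm each other to alternate press and release.
; Both the re-arming and the door calls require a valid light reference, so a button without one cycles only once.
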(event OnComponentBeginOverlap(Overlap)
  (params (OverlappedComponent :type Primitive%20Component%20Object%20Reference) (OtherActor :type Actor%20Object%20Reference) (OtherComp :type Primitive%20Component%20Object%20Reference) (OtherBodyIndex :type Integer) (bFromSweep :type Boolean) (SweepResult :type Hit%20Result%20Structure%20%28by%20ref%29))
  ;[1 1 1] Button
  (Utilities|Casting|CastToShape OtherActor)
  (Utilities|FlowControl|DoOnce false
    (:Completed
      (Audio|PlaySound2D "/Game/Sounds/Item_Collected.Item_Collected" 1.0 1.0 0.0 0 0)
      (Rendering|Components|Sprite|SetSprite (Variables|Default|GetButton) (Variables|Default|GetPressed_Sprite))
      (Utilities|IsValid (Variables|Default|GetButtonLight_Ref)
        (:Is%20Valid
          (Rendering|Components|Sprite|SetSprite (Variables|/Game/Levels/Actors/BP_ButtonLight.BP_ButtonLight_C|GetButtonLight (Variables|Default|GetButtonLight_Ref)) (Variables|/Game/Levels/Actors/BP_ButtonLight.BP_ButtonLight_C|GetLight_On (Variables|Default|GetButtonLight_Ref)))
          (CallFunction|ResetEndOverlap)
          (Utilities|IsValid (Variables|Default|GetDoorRef)
            (:Is%20Valid
              (Default|Open (Variables|Default|GetDoorRef)))))))))

(event OnComponentEndOverlap(Overlap)
  (params (OverlappedComponent :type Primitive%20Component%20Object%20Reference) (OtherActor :type Actor%20Object%20Reference) (OtherComp :type Primitive%20Component%20Object%20Reference) (OtherBodyIndex :type Integer))
  ;[1 1 1] Button
  (Utilities|Casting|CastToShape OtherActor)
  (Utilities|FlowControl|DoOnce false
    (:Completed
      (Audio|PlaySound2D "/Engine/EditorSounds/GamePreview/StartSimulate.StartSimulate" 1.0 1.0 0.0 0 0)
      (Rendering|Components|Sprite|SetSprite (Variables|Default|GetButton) (Variables|Default|GetUnpressed_Sprite))
      (Utilities|IsValid (Variables|Default|GetButtonLight_Ref)
        (:Is%20Valid
          (Rendering|Components|Sprite|SetSprite (Variables|/Game/Levels/Actors/BP_ButtonLight.BP_ButtonLight_C|GetButtonLight (Variables|Default|GetButtonLight_Ref)) (Variables|/Game/Levels/Actors/BP_ButtonLight.BP_ButtonLight_C|GetLight_Off (Variables|Default|GetButtonLight_Ref)))
          (CallFunction|ResetOverlap)
          (Utilities|IsValid (Variables|Default|GetDoorRef)
            (:Is%20Valid
              (Default|Close (Variables|Default|GetDoorRef)))))))))

(event Custom|Reset%20Overlap
  ;[1 1 1] Button
  (Utilities|FlowControl|DoOnce false) ; enters at Reset
)

(event Custom|Reset%20End%20Overlap
  ;[1 1 1] Button
  (Utilities|FlowControl|DoOnce false) ; enters at Reset
)

(event EventBeginPlay
  ;[1 1 1] Update to correct color
  (Rendering|Components|Sprite|SetSprite (Variables|Default|GetButton) (Variables|Default|GetUnpressed_Sprite)))

(fn ConstructionScript)