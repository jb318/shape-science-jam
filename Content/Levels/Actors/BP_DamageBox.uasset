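; Damage box actor that hurts Shape actors while they overlap its Box component, with configurable damage and an instant-kill option.
; Beginning overlap stores the Shape and, through a DoOnce, damages it immediately and starts a looping timer that re-applies damage.
; The stored Shape leaving clears the timer and resets the DoOnce.
; Only one Shape is tracked, so later entrants replace the timer's target.
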(event OnComponentBeginOverlap(Box)
  (params (OverlappedComponent :type Primitive%20Component%20Object%20Reference) (OtherActor :type Actor%20Object%20Reference) (OtherComp :type Primitive%20Component%20Object%20Reference) (OtherBodyIndex :type Integer) (bFromSweep :type Boolean) (SweepResult :type Hit%20Result%20Structure%20%28by%20ref%29))
  ;[1 1 1] Get damage type and call damage function on shape
  (bind _asshape (Utilities|Casting|CastToShape OtherActor))
  (Variables|Default|SetOverlapped%20Shape _asshape)
  (Utilities|FlowControl|DoOnce false
    (:Completed
      (Class|Shape|DamageShape (Variables|Default|GetOverlapped%20Shape) (Variables|Default|GetDamage) (Variables|Default|GetInstantKill))
      (Utilities|Time|SetTimerbyFunctionName 0 "ApplyDamageToShape" 1.5 true))))

(event OnComponentEndOverlap(Box)
  (params (OverlappedComponent :type Primitive%20Component%20Object%20Reference) (OtherActor :type Actor%20Object%20Reference) (OtherComp :type Primitive%20Component%20Object%20Reference) (OtherBodyIndex :type Integer))
  ;[1 1 1] Get damage type and call damage function on shape
  (if (== OtherActor (Variables|Default|GetOverlapped%20Shape))
    (Variables|Default|SetOverlapped%20Shape (Variables|Default|GetOverlapped%20Shape))
    (Utilities|Time|ClearTimerbyFunctionName 0 "ApplyDamageToShape")
    (CallFunction|ResetDamageTimer)))

(event Custom|ApplyDamageToShape
  (bind _overlapped_shape (Variables|Default|GetOverlapped%20Shape))
  ;[1 1 1] Get damage type and call damage function on shape
  (Utilities|IsValid _overlapped_shape
    (:Is%20Valid
      (Class|Shape|DamageShape _overlapped_shape (Variables|Default|GetDamage) (Variables|Default|GetInstantKill)))))

(event Custom|Reset%20Damage%20Timer
  ;[1 1 1] Get damage type and call damage function on shape
  (Utilities|FlowControl|DoOnce false) ; enters at Reset
)

(fn ConstructionScript)