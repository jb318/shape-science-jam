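; BP_Multiplayergamemode is a multiplayer game mode Blueprint with Server and Client events for player setup.
; BeginPlay switches the view mode to Unlit.
; Both events re-ID the player controller at index 0, Server to the first controller ID and Client to the second.
; Each also assigns its spawn variable, FirstPlayerSpawn or SecondPlayerSpawn, to itself, and no spawning occurs in the graph.
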(event Custom|Server
  (Variables|Default|SetFirstPlayerSpawn (Variables|Default|GetFirstPlayerSpawn))
  (Class|GameplayStatics|SetPlayerControllerID (Game|GetPlayerController 0)))

(event Custom|Client
  (Variables|Default|SetSecondPlayerSpawn (Variables|Default|GetSecondPlayerSpawn))
  (Class|GameplayStatics|SetPlayerControllerID (Game|GetPlayerController 0) 1))

(event EventBeginPlay
  (Class|Rendering|SetViewMode "VMI_Unlit"))

(fn ConstructionScript)