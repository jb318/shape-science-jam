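; BP_GameMode is a game mode Blueprint with unfinished logic for tracking player controllers.
; PostLogin is empty; unconnected nodes would count players, store each BP_PlayerController in AllShapeControllers and start a timer to call ChangePC.
; ChangePC checks whether the array's last index is 1 and loops over it, but its branch for the first entry does nothing.
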(event Custom|ChangePC
  (if (== (Utilities|Array|LastIndex (Variables|Default|GetAllShapeControllers)) 1)
    (for (_ _array_index) (Variables|Default|GetAllShapeControllers)
      (if (== _array_index 0)
        _))))

(event EventPostLogin
  (params (NewPlayer :type Player%20Controller%20Object%20Reference)))

(fn ConstructionScript)