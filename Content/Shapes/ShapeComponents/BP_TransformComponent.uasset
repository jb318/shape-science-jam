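; Shape component that sets its owning actor's transform, intended for network replication.
; TransformActor stores location, rotation and scale, then passes them through ServerTransform to MulticastShapeTransform, which applies them with SetActorTransform.
; The server event also prints a debug "Hello" when the owner is a BP_Circle.
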(event Custom|MulticastShapeTransform
  (params (Location :type Vector) (Rotation :type Rotator) (Scale :type Vector :default "1.000000,1.000000,1.000000"))
  ;[1 1 1] Shape Transform and Network Replication
  (Transformation|SetActorTransform (Components|GetOwner) (Math|Transform|MakeTransform Location Rotation Scale)))

(event Custom|ServerTransform
  (params (Location :type Vector) (Rotation :type Rotator) (Scale :type Vector :default "1.000000,1.000000,1.000000"))
  ;[1 1 1] Shape Transform and Network Replication
  (Utilities|Casting|CastToBP_Circle (Components|GetOwner)
    (:then
      (Development|PrintString "Hello"))
    (:CastFailed
      _))
  (CallFunction|MulticastShapeTransform (Variables|Default|GetLocation) (Variables|Default|GetRotation) (Variables|Default|GetScale)))

(event EventTransformActor
  (params (Location :type Vector :default "0, 0, 0") (Rotation :type Rotator :default "0, 0, 0") (Scale :type Vector :default "0, 0, 0"))
  ;[1 1 1] Shape Transform and Network Replication
  (bind _output_get (Variables|Default|SetLocation Location))
  (bind _output_get_2 (Variables|Default|SetRotation Rotation))
  (bind _output_get_3 (Variables|Default|SetScale Scale))
  (CallFunction|ServerTransform _output_get _output_get_2 _output_get_3))