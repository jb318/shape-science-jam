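; BP_ShapeAbilityComponent is an actor component that handles a Shape character's transforms and special move in multiplayer.
; Each ability routes a call through a server event to a multicast, which sets the actor's transform or plays Paper2D flipbooks before returning to idle.
; The special move requires enabled input and no falling, while transform-in re-enables input and movement afterwards.
; The Shape reference comes from the owner, cached two seconds after BeginPlay.
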(event Custom|MulticastShapeTransform
  (params (Location :type Vector) (Rotation :type Rotator) (Scale :type Vector :default "1.000000,1.000000,1.000000"))
  ;[1 1 1] Shape Transform and Network Replication
  (Transformation|SetActorTransform (Components|GetOwner) (Math|Transform|MakeTransform Location Rotation Scale)))

(event Custom|TransformOutServerCall
  ;[1 1 1] Shape Transform
  (CallFunction|TransformOutMulticast))

(event Custom|TransformOutMulticast
  (bind _shaperef (Variables|Default|GetShapeRef))
  (bind _shaperef_2 (Variables|Default|GetShapeRef))
  ;[1 1 1] Shape Transform
  (Utilities|FlowControl|DoOnce false :!label _label
    (:Completed
      (Sprite|SetFlipbook (Variables|/Script/Paper2D.PaperCharacter|GetSprite _shaperef) (Variables|/Script/shape_science_jam.Shape|GetTransformOutAnimation _shaperef))
      (Utilities|FlowControl|Delay 1.0)
      (Sprite|SetFlipbook (Variables|/Script/Paper2D.PaperCharacter|GetSprite _shaperef_2) (Variables|/Script/shape_science_jam.Shape|GetIdleAnimation _shaperef_2))
      (goto _label Reset))))

(event Custom|ServerTransform
  (params (Location :type Vector) (Rotation :type Rotator) (Scale :type Vector :default "1.000000,1.000000,1.000000"))
  ;[1 1 1] Shape Transform and Network Replication
  (bind _asshape (Utilities|Casting|CastToShape (Components|GetOwner)))
  (Variables|Default|SetShapeRef _asshape)
  (CallFunction|MulticastShapeTransform (Variables|Default|GetLocation) (Variables|Default|GetRotation) (Variables|Default|GetScale)))

(event Custom|TransformInServerCall
  ;[1 1 1] Shape Transform
  (CallFunction|TransforminMulticast))

(event Custom|TransformInMulticast
  (bind _shaperef (Variables|Default|GetShapeRef))
  (bind _shaperef_2 (Variables|Default|GetShapeRef))
  (bind _shaperef_3 (Variables|Default|GetShapeRef))
  ;[1 1 1] Shape Transform
  (Sprite|SetFlipbook (Variables|/Script/Paper2D.PaperCharacter|GetSprite _shaperef_2) (Variables|/Script/shape_science_jam.Shape|GetTransformInAnimation _shaperef_2))
  (Utilities|FlowControl|Delay 0.667)
  (Sprite|SetFlipbook (Variables|/Script/Paper2D.PaperCharacter|GetSprite _shaperef_3) (Variables|/Script/shape_science_jam.Shape|GetIdleAnimation _shaperef_3))
  (Variables|/Script/shape_science_jam.Shape|SetInputDisabled _shaperef false)
  (Variables|/Script/shape_science_jam.Shape|SetCannotMove _shaperef false))

(event Custom|SpecialMoveServerCall
  ;[1 1 1] Shape Special Move
  (CallFunction|SpecialMoveMulticast))

(event Custom|SpecialMoveMulticast
  (bind _shaperef (Variables|Default|GetShapeRef))
  (bind _shaperef_2 (Variables|Default|GetShapeRef))
  ;[1 1 1] Shape Special Move
  (Utilities|IsValid _shaperef_2
    (:Is%20Valid
      (Sprite|SetFlipbook (Variables|/Script/Paper2D.PaperCharacter|GetSprite _shaperef_2) (Variables|/Script/shape_science_jam.Shape|GetSpecialMoveAnimation _shaperef_2))
      (Utilities|FlowControl|Delay (Variables|/Script/shape_science_jam.Shape|GetSpecialMoveAnimationDuration _shaperef))
      (Sprite|SetFlipbook (Variables|/Script/Paper2D.PaperCharacter|GetSprite _shaperef) (Variables|/Script/shape_science_jam.Shape|GetIdleAnimation _shaperef))
      (Variables|/Script/shape_science_jam.Shape|SetInputDisabled (Variables|Default|GetShapeRef) false))))

(event EventBeginPlay
  ;[1 1 1] Sets shape ref in net multiplayer
  (Utilities|FlowControl|Delay 2.0)
  (bind _asshape (Utilities|Casting|CastToShape (Components|GetOwner)))
  (Variables|Default|SetShapeRef _asshape))

(event EventTransformOutAnimationCall
  ;[1 1 1] Shape Transform
  (CallFunction|TransformOutServerCall))

(event EventTransformActor
  (params (Location :type Vector :default "0, 0, 0") (Rotation :type Rotator :default "0, 0, 0") (Scale :type Vector :default "0, 0, 0"))
  ;[1 1 1] Shape Transform and Network Replication
  (bind _output_get (Variables|Default|SetLocation Location))
  (bind _output_get_2 (Variables|Default|SetRotation Rotation))
  (bind _output_get_3 (Variables|Default|SetScale Scale))
  (CallFunction|ServerTransform _output_get _output_get_2 _output_get_3))

(event EventSpecialMoveAnimationCall
  (bind _shaperef (Variables|Default|GetShapeRef))
  ;[1 1 1] Shape Special Move
  (Utilities|IsValid _shaperef
    (:Is%20Valid
      (if (not (Variables|/Script/shape_science_jam.Shape|GetInputDisabled _shaperef))
        (if (not (AI|Components|NavMovement|IsFalling (Variables|/Script/Engine.Character|GetCharacterMovement (Variables|Default|GetShapeRef))))
          (CallFunction|SpecialMoveServerCall)
          (Development|PrintString "Hello"))))))

(event EventTransforminAnimationCall
  ;[1 1 1] Shape Transform
  (CallFunction|TransforminServerCall))