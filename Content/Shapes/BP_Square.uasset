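; Player square shape character, handling its movement, reflect attack, gravity-flip special, damage and shape-change animations.
; Input and gameplay events swap Paper2D flipbooks, with state flags and Delays gating actions and freezing walk speed during both moves.
; Reflect grants temporary projectile immunity; the special only rotates the sprite from UsingAntiGravity, without changing gravity here.
; A one-second timer after BeginPlay sets the counter projectiles' flipbooks to the enemy triangle idle.
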(event Custom|ChangeFlipbook
  (bind _projectile1 (Variables|Default|GetProjectile1))
  (bind _projectile2 (Variables|Default|GetProjectile2))
  ;[1 1 1] Sets flipbook of counter projectile
  (Utilities|IsValid _projectile1
    (:Is%20Valid
      (Sprite|SetFlipbook (Variables|/Script/shape_science_jam.Projectile|GetFlipbook _projectile1) "/Game/Import_Assets/Sprites/EnemyTriangle/Animations/EnemyTriangle_RightIdle.EnemyTriangle_RightIdle")
      (Utilities|IsValid _projectile2
        (:Is%20Valid
          (Sprite|SetFlipbook (Variables|/Script/shape_science_jam.Projectile|GetFlipbook _projectile2) "/Game/Import_Assets/Sprites/EnemyTriangle/Animations/EnemyTriangle_RightIdle.EnemyTriangle_RightIdle"))))))

(event Input|EnhancedActionEvents|EnhancedInputActionIA_Move
  (params (ActionValue :type Float%20%28double-precision%29) (ElapsedSeconds :type Float%20%28double-precision%29) (TriggeredSeconds :type Float%20%28double-precision%29) (InputAction :type Input%20Action%20Object%20Reference :default "/Game/Inputs/IA_Move.IA_Move"))
  (bind _indamagecooldown (Variables|Default|GetInDamageCoolDown))
  (bind _inspecialattackanimation (Variables|Default|GetInSpecialAttackAnimation))
  (bind _charactermovement (Variables|Character|GetCharacterMovement))
  (bind _changingshape (Variables|Default|GetChangingShape))
  (bind _returnvalue (AI|Components|NavMovement|IsFalling _charactermovement))
  (bind _returnvalue_2 (or _indamagecooldown _changingshape))
  ;[1 1 1] Square movement animation
  (:Triggered
    (if (not _returnvalue_2)
      (if (not (AI|Components|NavMovement|IsFalling (Variables|Character|GetCharacterMovement)))
        (if (not (or (Variables|Default|GetInAttackAnimation) (Variables|Default|GetInSpecialAttackAnimation)))
          (Sprite|SetFlipbook (Variables|Default|GetSprite) "/Game/Import_Assets/Sprites/PlayerSquares/Animations/PlayerSquare_Moving.PlayerSquare_Moving")
          (if (> ActionValue 0.0)
            (if (not (Variables|Default|GetFacingRight))
              (Transformation|SetRelativeRotation (Variables|Default|GetSprite) "0, 0, 0" false false)
              (Variables|Default|SetFacingLeft false)
              (Variables|Default|SetFacingRight true))
            (elif (not (Variables|Default|GetFacingLeft))
              (Transformation|SetRelativeRotation (Variables|Default|GetSprite) "0.000000,180.000000,0.000000" false false)
              (Variables|Default|SetFacingLeft true)
              (Variables|Default|SetFacingRight false)))))))
  (:Started
    (if (not _returnvalue_2)
      (if (not _returnvalue)
        (if (not (or (Variables|Default|GetInAttackAnimation) _inspecialattackanimation))
          (Sprite|SetFlipbook (Variables|Default|GetSprite) "/Game/Import_Assets/Sprites/PlayerSquares/Animations/PlayerSquare_StartMoving.PlayerSquare_StartMoving")))))
  (:Completed
    (if (not _returnvalue_2)
      (if (not _returnvalue)
        (if (not (or _inspecialattackanimation (Variables|Default|GetInAttackAnimation)))
          (Sprite|SetFlipbook (Variables|Default|GetSprite) "/Game/Import_Assets/Sprites/PlayerSquares/Animations/PlayerSquare_FinishMoving.PlayerSquare_FinishMoving")
          (Sprite|SetFlipbook (Variables|Default|GetSprite) "/Game/Import_Assets/Sprites/PlayerSquares/Animations/Square_Standby.Square_Standby"))))))

(event EventChangeShapeStart
  ;[1 1 1] Change shape animations
  (if (not (Variables|Default|GetChangingShape))
    (if (Variables|Default|GetCanChangeShape)
      (Sprite|SetFlipbook (Variables|Default|GetSprite) "/Game/Import_Assets/Sprites/PlayerSquares/Animations/PlayerSquare_Transform_out.PlayerSquare_Transform_out")
      (Variables|Default|SetChangingShape true))))

(event EventPlayDamageAnimation
  ;[1 1 1] Plays damage animation
  (if (not (Variables|Default|GetImmuneToProjectile))
    (Variables|Default|SetInDamageCoolDown true)
    (Variables|Default|SetCanChangeShape false)
    (Sprite|SetFlipbook (Variables|Default|GetSprite) "/Game/Import_Assets/Sprites/PlayerSquares/Animations/PlayerSquare_Hit.PlayerSquare_Hit")
    (Utilities|FlowControl|Delay 0.5)
    (Variables|Default|SetInDamageCoolDown false)
    (Sprite|SetFlipbook (Variables|Default|GetSprite) "/Game/Import_Assets/Sprites/PlayerSquares/Animations/Square_Standby.Square_Standby")
    (Variables|Default|SetCanChangeShape true)))

(event EventChangeShapeEnd
  ;[1 1 1] Change shape animations
  (Variables|Default|SetChangingShape true)
  (Sprite|SetFlipbook (Variables|Default|GetSprite) "/Game/Import_Assets/Sprites/PlayerSquares/Animations/PlayerSquare_Transform_in.PlayerSquare_Transform_in")
  (Utilities|FlowControl|Delay 0.667)
  (Variables|Default|SetChangingShape false)
  (Sprite|SetFlipbook (Variables|Default|GetSprite) "/Game/Import_Assets/Sprites/PlayerSquares/Animations/Square_Standby.Square_Standby"))

(event EventAttack
  ;[1 1 1] Attack animation
  (if (not (Variables|Default|GetCoolDownActive))
    (Variables|Default|SetInAttackAnimation true)
    (Variables|Default|SetImmuneToProjectile true)
    (Sprite|SetFlipbook (Variables|Default|GetSprite) "/Game/Import_Assets/Sprites/PlayerSquares/Animations/PlayerSquare_Reflect.PlayerSquare_Reflect")
    (Variables|/Script/Engine.CharacterMovementComponent|SetMaxWalkSpeed (Variables|Character|GetCharacterMovement) 0.0)
    (Utilities|FlowControl|Delay 1.0)
    (Variables|/Script/Engine.CharacterMovementComponent|SetMaxWalkSpeed (Variables|Character|GetCharacterMovement) 6e+02)
    (Sprite|SetFlipbook (Variables|Default|GetSprite) "/Game/Import_Assets/Sprites/PlayerSquares/Animations/Square_Standby.Square_Standby")
    (Variables|Default|SetInAttackAnimation false)
    (Variables|Default|SetImmuneToProjectile false)))

(event EventSpecialMove
  (bind _sprite (Variables|Default|GetSprite))
  (bind _sprite_2 (Variables|Default|GetSprite))
  ;[1 1 1] Square anti-gravity
  (if (not (Variables|Default|GetInAttackAnimation))
    (Variables|Default|SetInSpecialAttackAnimation true)
    (Variables|/Script/Engine.CharacterMovementComponent|SetMaxWalkSpeed (Variables|Character|GetCharacterMovement) 0.0)
    (Sprite|SetFlipbook (Variables|Default|GetSprite) "/Game/Import_Assets/Sprites/PlayerSquares/Animations/PlayerSquare_FlipGravity.PlayerSquare_FlipGravity")
    (Utilities|FlowControl|Delay 1.0)
    (Variables|Default|SetInSpecialAttackAnimation false)
    (Variables|/Script/Engine.CharacterMovementComponent|SetMaxWalkSpeed (Variables|Character|GetCharacterMovement) 6e+02)
    (if (Variables|Default|GetUsingAntiGravity)
      (Transformation|SetWorldRotation _sprite_2 "180.000000,0.000000,0.000000" false false)
      (Sprite|SetFlipbook _sprite "/Game/Import_Assets/Sprites/PlayerSquares/Animations/Square_Standby.Square_Standby")
      (else
        (Transformation|SetWorldRotation _sprite_2 "0, 0, 0" false false)
        (Sprite|SetFlipbook _sprite "/Game/Import_Assets/Sprites/PlayerSquares/Animations/Square_Standby.Square_Standby")))))

(event EventBeginPlay
  ;[1 1 1] Sets flipbook of counter projectile
  (Utilities|Time|SetTimerbyFunctionName 0 "ChangeFlipbook" 1.0))

(fn ConstructionScript)