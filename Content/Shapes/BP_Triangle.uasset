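; Triangle player shape Blueprint that drives flipbook animations for turning, attacking, taking damage and transforming between shapes.
; Move input rotates the sprite to face the travel direction, reusing a single turn flipbook for both sides.
; Attack runs only off cooldown and while not falling, briefly zeroing walk speed.
; State flags and timed Delays block movement animations during attacks, hits and transforms, and attacks and hits also block shape changes.
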(event Input|EnhancedActionEvents|EnhancedInputActionIA_Move
  (params (ActionValue :type Float%20%28double-precision%29) (ElapsedSeconds :type Float%20%28double-precision%29) (TriggeredSeconds :type Float%20%28double-precision%29) (InputAction :type Input%20Action%20Object%20Reference :default "/Game/Inputs/IA_Move.IA_Move"))
  (bind _indamagecooldown (Variables|Default|GetInDamageCoolDown))
  (bind _changingshape (Variables|Default|GetChangingShape))
  (bind _inattackanimation (Variables|Default|GetInAttackAnimation))
  (bind _returnvalue (Math|Boolean|ORBoolean _inattackanimation _indamagecooldown _changingshape))
  ;[1 1 1] Movement animations
  (:Triggered
    (if (not _returnvalue)
      (if (> ActionValue 0.0)
        (if (not (Variables|Default|GetFacingRight))
          (Transformation|SetRelativeRotation (Variables|Default|GetSprite) "0, 0, 0" false false)
          (Variables|Default|SetFacingRight true)
          (Variables|Default|SetFacingLeft false)
          (Sprite|SetFlipbook (Variables|Default|GetSprite) "/Game/Import_Assets/Sprites/PlayerTriangle/Animations/PlayerTriangle_RotateRight.PlayerTriangle_RotateRight")
          (Utilities|FlowControl|Delay 0.333)
          (Sprite|SetFlipbook (Variables|Default|GetSprite) "/Game/Import_Assets/Sprites/PlayerTriangle/Animations/PlayerTriangle_RightIdle.PlayerTriangle_RightIdle"))
        (elif (< ActionValue 0.0)
          (if (not (Variables|Default|GetFacingLeft))
            (Transformation|SetRelativeRotation (Variables|Default|GetSprite) "0.000000,180.000000,0.000000" false false)
            (Variables|Default|SetFacingRight false)
            (Variables|Default|SetFacingLeft true)
            (Sprite|SetFlipbook (Variables|Default|GetSprite) "/Game/Import_Assets/Sprites/PlayerTriangle/Animations/PlayerTriangle_RotateRight.PlayerTriangle_RotateRight")
            (Utilities|FlowControl|Delay 0.333)
            (Sprite|SetFlipbook (Variables|Default|GetSprite) "/Game/Import_Assets/Sprites/PlayerTriangle/Animations/PlayerTriangle_RightIdle.PlayerTriangle_RightIdle"))))))
  (:Completed
    (if (not _returnvalue)
      (Sprite|SetFlipbook (Variables|Default|GetSprite) "/Game/Import_Assets/Sprites/PlayerTriangle/Animations/PlayerTriangle_RightIdle.PlayerTriangle_RightIdle"))))

(event EventChangeShapeStart
  ;[1 1 1] Change shape animations
  (if (not (Variables|Default|GetChangingShape))
    (if (Variables|Default|GetCanChangeShape)
      (Sprite|SetFlipbook (Variables|Default|GetSprite) "/Game/Import_Assets/Sprites/PlayerTriangle/Animations/PlayerTriangle_TransformOut.PlayerTriangle_TransformOut")
      (Variables|Default|SetChangingShape true))))

(event EventPlayDamageAnimation
  ;[1 1 1] Plays damage animation
  (Variables|Default|SetInDamageCoolDown true)
  (Variables|Default|SetCanChangeShape false)
  (Sprite|SetFlipbook (Variables|Default|GetSprite) "/Game/Import_Assets/Sprites/PlayerTriangle/Animations/PlayerTriangle_Hit.PlayerTriangle_Hit")
  (Utilities|FlowControl|Delay 0.5)
  (Sprite|SetFlipbook (Variables|Default|GetSprite) "/Game/Import_Assets/Sprites/PlayerTriangle/Animations/PlayerTriangle_RightIdle.PlayerTriangle_RightIdle")
  (Variables|Default|SetInDamageCoolDown false)
  (Variables|Default|SetCanChangeShape true))

(event EventChangeShapeEnd
  ;[1 1 1] Change shape animations
  (Variables|Default|SetChangingShape true)
  (Sprite|SetFlipbook (Variables|Default|GetSprite) "/Game/Import_Assets/Sprites/PlayerTriangle/Animations/PlayerTriangle_TransformIn.PlayerTriangle_TransformIn")
  (Utilities|FlowControl|Delay 0.667)
  (Variables|Default|SetChangingShape false)
  (Sprite|SetFlipbook (Variables|Default|GetSprite) "/Game/Import_Assets/Sprites/PlayerTriangle/Animations/PlayerTriangle_RightIdle.PlayerTriangle_RightIdle"))

(event EventAttack
  ;[1 1 1] Triangle Attack
  (if (and (not (Variables|Default|GetCoolDownActive)) (not (AI|Components|NavMovement|IsFalling (Variables|Character|GetCharacterMovement))))
    (Variables|Default|SetInAttackAnimation true)
    (Variables|Default|SetCanChangeShape false)
    (Sprite|SetFlipbook (Variables|Default|GetSprite) "/Game/Import_Assets/Sprites/PlayerTriangle/Animations/PlayerTriangle_Attack.PlayerTriangle_Attack")
    (Variables|/Script/Engine.CharacterMovementComponent|SetMaxWalkSpeed (Variables|Character|GetCharacterMovement) 0.0)
    (Utilities|FlowControl|Delay 0.5)
    (Variables|/Script/Engine.CharacterMovementComponent|SetMaxWalkSpeed (Variables|Character|GetCharacterMovement) 6e+02)
    (Sprite|SetFlipbook (Variables|Default|GetSprite) "/Game/Import_Assets/Sprites/PlayerTriangle/Animations/PlayerTriangle_RightIdle.PlayerTriangle_RightIdle")
    (Variables|Default|SetInAttackAnimation false)
    (Variables|Default|SetCanChangeShape true)))

(fn ConstructionScript)