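; BP_Star is the playable star shape, handling its Paper2D flipbook animations for walking, attacking, taking damage, the glide special move and shape changes.
; Movement input flips the sprite by facing, while delay-timed sequences return to idle or clear state flags such as InputDisabled.
; Attack and shape changes play locally and go through server-request events to multicasts, whereas damage and glide animations have no such relay here.
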(event Custom|MulticastShapeChangeOut
  ;[1 1 1] Change shape animations
  (if (Variables|Default|GetInputDisabled)
    (Utilities|FlowControl|DoOnce false :!label _label
      (:Completed
        (Sprite|SetFlipbook (Variables|Default|GetSprite) "/Game/Import_Assets/Sprites/PlayerStar/Animations/PlayerStar_TransformOut.PlayerStar_TransformOut")
        (Utilities|FlowControl|Delay 1.0)
        (Sprite|SetFlipbook (Variables|Default|GetSprite) "/Game/Import_Assets/Sprites/PlayerStar/Animations/PlayerStar_Idle.PlayerStar_Idle")
        (goto _label Reset)))))

(event Custom|ShapeChangeOutServerRequest
  ;[1 1 1] Change shape animations
  (CallFunction|MulticastShapeChangeOut))

(event Custom|ShapeChangeInServerRequest
  ;[1 1 1] Change shape animations
  (CallFunction|MulticastShapeChangein))

(event Custom|MulticastShapeChangeIn
  ;[1 1 1] Change shape animations
  (Sprite|SetFlipbook (Variables|Default|GetSprite) "/Game/Import_Assets/Sprites/PlayerStar/Animations/PlayerStar_TransformIn.PlayerStar_TransformIn")
  (Utilities|FlowControl|Delay 0.667)
  (Variables|Default|SetInputDisabled false)
  (Sprite|SetFlipbook (Variables|Default|GetSprite) "/Game/Import_Assets/Sprites/PlayerStar/Animations/PlayerStar_Idle.PlayerStar_Idle")
  (Variables|Default|SetCannotMove false))

(event Custom|AttackServerRequest
  ;[1 1 1] Star attack
  (CallFunction|MulticastAttack))

(event Custom|MulticastAttack
  ;[1 1 1] Star attack
  (if (not (Variables|Default|GetSpecialMoveClicked))
    (if (not (Variables|Default|GetCoolDownActive))
      (if (not (AI|Components|NavMovement|IsFalling (Variables|Character|GetCharacterMovement)))
        (if (not (Variables|Default|GetInputDisabled))
          (Sprite|SetFlipbook (Variables|Default|GetSprite) "/Game/Import_Assets/Sprites/PlayerStar/Animations/PlayerStar_Attack.PlayerStar_Attack")
          (Utilities|FlowControl|Delay 0.25)
          (Sprite|SetFlipbook (Variables|Default|GetSprite) "/Game/Import_Assets/Sprites/PlayerStar/Animations/PlayerStar_Idle.PlayerStar_Idle")
          (Variables|Default|SetInputDisabled false))))))

(event Input|EnhancedActionEvents|EnhancedInputActionIA_Move
  (params (ActionValue :type Float%20%28double-precision%29) (ElapsedSeconds :type Float%20%28double-precision%29) (TriggeredSeconds :type Float%20%28double-precision%29) (InputAction :type Input%20Action%20Object%20Reference :default "/Game/Inputs/IA_Move.IA_Move"))
  (bind _inputdisabled (Variables|Default|GetInputDisabled))
  ;[1 1 1] Movement animations
  (:Triggered
    (if (not _inputdisabled)
      (if (not (AI|Components|NavMovement|IsFalling (Variables|Character|GetCharacterMovement)))
        (if (> ActionValue 0.0)
          (Sprite|SetFlipbook (Variables|Default|GetSprite) "/Game/Import_Assets/Sprites/PlayerStar/Animations/PlayerStar_Walk.PlayerStar_Walk")
          (if (not (Variables|Default|GetFacingRight))
            (Transformation|SetRelativeRotation (Variables|Default|GetSprite) "0, 0, 0" false false)
            (Variables|Default|SetFacingRight true)
            (Variables|Default|SetFacingLeft false))
          (elif (< ActionValue 0.0)
            (Sprite|SetFlipbook (Variables|Default|GetSprite) "/Game/Import_Assets/Sprites/PlayerStar/Animations/PlayerStar_Walk.PlayerStar_Walk")
            (if (not (Variables|Default|GetFacingLeft))
              (Transformation|SetRelativeRotation (Variables|Default|GetSprite) "0.000000,180.000000,0.000000" false false)
              (Variables|Default|SetFacingRight false)
              (Variables|Default|SetFacingLeft true)))))))
  (:Completed
    (if (not _inputdisabled)
      (Sprite|SetFlipbook (Variables|Default|GetSprite) "/Game/Import_Assets/Sprites/PlayerStar/Animations/PlayerStar_Idle.PlayerStar_Idle"))))

(event EventChangeShapeStart
  ;[1 1 1] Change shape animations
  (CallFunction|ShapeChangeOutServerRequest)
  (if (Variables|Default|GetInputDisabled)
    (Utilities|FlowControl|DoOnce false :!label _label
      (:Completed
        (Sprite|SetFlipbook (Variables|Default|GetSprite) "/Game/Import_Assets/Sprites/PlayerStar/Animations/PlayerStar_TransformOut.PlayerStar_TransformOut")
        (Utilities|FlowControl|Delay 1.0)
        (Sprite|SetFlipbook (Variables|Default|GetSprite) "/Game/Import_Assets/Sprites/PlayerStar/Animations/PlayerStar_Idle.PlayerStar_Idle")
        (goto _label Reset)))))

(event EventSpecialMove
  ;[1 1 1] Glide
  (Sprite|SetFlipbook (Variables|Default|GetSprite) "/Game/Import_Assets/Sprites/PlayerStar/Animations/PlayerStar_Idle.PlayerStar_Idle")
  (Utilities|FlowControl|Delay (Variables|Default|GetSpecialMoveDelay))
  (Sprite|SetFlipbook (Variables|Default|GetSprite) "/Game/Import_Assets/Sprites/PlayerStar/Animations/PlayerStar_Launched.PlayerStar_Launched")
  (Utilities|FlowControl|Delay 0.24)
  (Sprite|SetFlipbook (Variables|Default|GetSprite) "/Game/Import_Assets/Sprites/PlayerStar/Animations/PlayerStar_Idle.PlayerStar_Idle")
  (Utilities|FlowControl|Delay 0.11)
  (Variables|Default|SetInputDisabled false)
  (Variables|Default|SetSpecialMoveClicked false))

(event EventChangeShapeEnd
  ;[1 1 1] Change shape animations
  (CallFunction|ShapeChangeinServerRequest)
  (Sprite|SetFlipbook (Variables|Default|GetSprite) "/Game/Import_Assets/Sprites/PlayerStar/Animations/PlayerStar_TransformIn.PlayerStar_TransformIn")
  (Utilities|FlowControl|Delay 0.667)
  (Variables|Default|SetInputDisabled false)
  (Sprite|SetFlipbook (Variables|Default|GetSprite) "/Game/Import_Assets/Sprites/PlayerStar/Animations/PlayerStar_Idle.PlayerStar_Idle")
  (Variables|Default|SetCannotMove false))

(event EventPlayDamageAnimation
  ;[1 1 1] Plays damage animation
  (if (not (Variables|Default|GetInvincible))
    (Sprite|SetFlipbook (Variables|Default|GetSprite) "/Game/Import_Assets/Sprites/PlayerStar/Animations/PlayerStar_Hit.PlayerStar_Hit")
    (Utilities|FlowControl|Delay 0.5)
    (Sprite|SetFlipbook (Variables|Default|GetSprite) "/Game/Import_Assets/Sprites/PlayerStar/Animations/PlayerStar_Idle.PlayerStar_Idle")
    (Variables|Default|SetImmuneToProjectile false)
    (Variables|Default|SetInputDisabled false)))

(event EventAttack
  ;[1 1 1] Star attack
  (CallFunction|AttackServerRequest)
  (if (not (Variables|Default|GetSpecialMoveClicked))
    (if (not (Variables|Default|GetCoolDownActive))
      (if (not (AI|Components|NavMovement|IsFalling (Variables|Character|GetCharacterMovement)))
        (if (not (Variables|Default|GetInputDisabled))
          (Sprite|SetFlipbook (Variables|Default|GetSprite) "/Game/Import_Assets/Sprites/PlayerStar/Animations/PlayerStar_Attack.PlayerStar_Attack")
          (Utilities|FlowControl|Delay 0.25)
          (Sprite|SetFlipbook (Variables|Default|GetSprite) "/Game/Import_Assets/Sprites/PlayerStar/Animations/PlayerStar_Idle.PlayerStar_Idle")
          (Variables|Default|SetInputDisabled false))))))

(fn ConstructionScript)