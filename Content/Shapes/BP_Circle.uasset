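; Circle form of the shape-shifting player character, handling its flipbook animations and state flags for movement, attack, bounce, damage and transformation.
; Move input plays the rolling flipbook and rotates the sprite to face left or right unless shape change, damage cooldown or attack is active.
; Attack is a grounded dash animation that briefly zeroes walk speed and opens an enemy-hit window.
; Timed Delays restore idle and clear the flags.
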(event Input|EnhancedActionEvents|EnhancedInputActionIA_Move
  (params (ActionValue :type Float%20%28double-precision%29) (ElapsedSeconds :type Float%20%28double-precision%29) (TriggeredSeconds :type Float%20%28double-precision%29) (InputAction :type Input%20Action%20Object%20Reference :default "/Game/Inputs/IA_Move.IA_Move"))
  (bind _indamagecooldown (Variables|Default|GetInDamageCoolDown))
  (bind _changingshape (Variables|Default|GetChangingShape))
  (bind _inattackanimation (Variables|Default|GetInAttackAnimation))
  (bind _returnvalue (Math|Boolean|ORBoolean _changingshape _indamagecooldown _inattackanimation))
  ;[1 1 1] Circle movement animation control
  (:Triggered
    (if (not _returnvalue)
      (if (Variables|Default|GetJumpButtonPressed)
        (Sprite|SetFlipbook (Variables|Default|GetSprite) "/Game/Import_Assets/Sprites/PlayerCircles/Animations/PlayerCircle_Bounce.PlayerCircle_Bounce")
        (Utilities|FlowControl|Delay 0.25)
        (Sprite|SetFlipbook (Variables|Default|GetSprite) "/Game/Import_Assets/Sprites/PlayerCircles/Animations/PlayerCircle_Idle.PlayerCircle_Idle")
        (elif (> ActionValue 0.0)
          (Sprite|SetFlipbook (Variables|Default|GetSprite) "/Game/Import_Assets/Sprites/PlayerCircles/Animations/PlayerCircle_NormalRolling.PlayerCircle_NormalRolling")
          (if (not (Variables|Default|GetFacingRight))
            (Transformation|SetRelativeRotation (Variables|Default|GetSprite) "0, 0, 0" false false)
            (Variables|Default|SetFacingRight true)
            (Variables|Default|SetFacingLeft false))
          (elif (< ActionValue 0.0)
            (Sprite|SetFlipbook (Variables|Default|GetSprite) "/Game/Import_Assets/Sprites/PlayerCircles/Animations/PlayerCircle_NormalRolling.PlayerCircle_NormalRolling")
            (if (not (Variables|Default|GetFacingLeft))
              (Transformation|SetRelativeRotation (Variables|Default|GetSprite) "0.000000,180.000000,0.000000" false false)
              (Variables|Default|SetFacingRight false)
              (Variables|Default|SetFacingLeft true)))))))
  (:Completed
    (if (not _returnvalue)
      (Sprite|SetFlipbook (Variables|Default|GetSprite) "/Game/Import_Assets/Sprites/PlayerCircles/Animations/PlayerCircle_Idle.PlayerCircle_Idle"))))

(event EventChangeShapeStart
  ;[1 1 1] Change shape animations
  (if (not (Variables|Default|GetChangingShape))
    (if (Variables|Default|GetCanChangeShape)
      (Sprite|SetFlipbook (Variables|Default|GetSprite) "/Game/Import_Assets/Sprites/PlayerCircles/Animations/PlayerCircle_TransformOut.PlayerCircle_TransformOut")
      (Variables|Default|SetChangingShape true))))

(event EventPlayDamageAnimation
  ;[1 1 1] Plays damage animation and temporarily halts inputs
  (Variables|Default|SetInDamageCoolDown true)
  (Variables|Default|SetCanChangeShape false)
  (Sprite|SetFlipbook (Variables|Default|GetSprite) "/Game/Import_Assets/Sprites/PlayerCircles/Animations/PlayerCircle_Hit.PlayerCircle_Hit")
  (Utilities|FlowControl|Delay 0.5)
  (Variables|Default|SetInDamageCoolDown false)
  (Sprite|SetFlipbook (Variables|Default|GetSprite) "/Game/Import_Assets/Sprites/PlayerCircles/Animations/PlayerCircle_Idle.PlayerCircle_Idle")
  (Variables|Default|SetCanChangeShape true))

(event EventChangeShapeEnd
  ;[1 1 1] Change shape animations
  (Variables|Default|SetChangingShape true)
  (Sprite|SetFlipbook (Variables|Default|GetSprite) "/Game/Import_Assets/Sprites/PlayerCircles/Animations/PlayerCircle_Transformin.PlayerCircle_TransformIn")
  (Utilities|FlowControl|Delay 0.667)
  (Variables|Default|SetChangingShape false)
  (Sprite|SetFlipbook (Variables|Default|GetSprite) "/Game/Import_Assets/Sprites/PlayerCircles/Animations/PlayerCircle_Idle.PlayerCircle_Idle"))

(event EventAttack
  ;[1 1 1] Speed dash attack animation handling
  (if (not (AI|Components|NavMovement|IsFalling (Variables|Character|GetCharacterMovement)))
    (Variables|/Script/Engine.CharacterMovementComponent|SetMaxWalkSpeed (Variables|Character|GetCharacterMovement) 0.0)
    (Variables|Default|SetInAttackAnimation true)
    (Variables|Default|SetCanChangeShape false)
    (Variables|Default|SetCanHitEnemy true)
    (Sprite|SetFlipbook (Variables|Default|GetSprite) "/Game/Import_Assets/Sprites/PlayerCircles/Animations/Playrer_CircleDash.Playrer_CircleDash")
    (Utilities|FlowControl|Delay 0.2)
    (Variables|/Script/Engine.CharacterMovementComponent|SetMaxWalkSpeed (Variables|Character|GetCharacterMovement) 6e+02)
    (Variables|Default|SetCanHitEnemy false)
    (Variables|Default|SetCanChangeShape true)
    (Sprite|SetFlipbook (Variables|Default|GetSprite) "/Game/Import_Assets/Sprites/PlayerCircles/Animations/PlayerCircle_Idle.PlayerCircle_Idle")
    (Variables|Default|SetInAttackAnimation false)))

(event EventSpecialMove
  ;[1 1 1] Circle jump
  (if (not (AI|Components|NavMovement|IsFalling (Variables|Character|GetCharacterMovement)))
    (Variables|Default|SetJumpButtonPressed true)
    (Sprite|SetFlipbook (Variables|Default|GetSprite) "/Game/Import_Assets/Sprites/PlayerCircles/Animations/PlayerCircle_Bounce.PlayerCircle_Bounce")
    (Utilities|FlowControl|Delay 0.25)
    (Sprite|SetFlipbook (Variables|Default|GetSprite) "/Game/Import_Assets/Sprites/PlayerCircles/Animations/PlayerCircle_Idle.PlayerCircle_Idle")
    (Variables|Default|SetJumpButtonPressed false)))

(fn ConstructionScript)