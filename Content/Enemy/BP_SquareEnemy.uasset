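; BP_SquareEnemy is a flipbook-animated square enemy that reverses on walls and ledges and reacts to shapes and their projectiles.
; Detector overlaps flip its facing, while Tick restores the walk flipbook and attack or hit events pause movement on timed delays.
; Its box triggers a mirror attack against Triangle projectiles, briefly drops projectile immunity for Star projectiles, and launches other Shapes in its facing direction.
; The damage calls on launched Shapes are unconnected.
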(event OnComponentBeginOverlap(WallDetector)
  (params (OverlappedComponent :type Primitive%20Component%20Object%20Reference) (OtherActor :type Actor%20Object%20Reference) (OtherComp :type Primitive%20Component%20Object%20Reference) (OtherBodyIndex :type Integer) (bFromSweep :type Boolean) (SweepResult :type Hit%20Result%20Structure%20%28by%20ref%29))
  ;[1 1 1] Turn
  (CallFunction|Turn))

(event OnComponentEndOverlap(LedgeDetector)
  (params (OverlappedComponent :type Primitive%20Component%20Object%20Reference) (OtherActor :type Actor%20Object%20Reference) (OtherComp :type Primitive%20Component%20Object%20Reference) (OtherBodyIndex :type Integer))
  ;[1 1 1] Turn
  (CallFunction|Turn))

(event OnComponentBeginOverlap(BoxComponent)
  (params (OverlappedComponent :type Primitive%20Component%20Object%20Reference) (OtherActor :type Actor%20Object%20Reference) (OtherComp :type Primitive%20Component%20Object%20Reference) (OtherBodyIndex :type Integer) (bFromSweep :type Boolean) (SweepResult :type Hit%20Result%20Structure%20%28by%20ref%29))
  ;[1 1 1] Reflect Triangles attacks
  (bind _asbp_triangle_projectile (Utilities|Casting|CastToBP_TriangleProjectile OtherActor)
    (:then
      (Utilities|Casting|CastToBP_Triangle (Game|GetInstigator _asbp_triangle_projectile))
      (Class|Shape|Attack))
    (:CastFailed
      (bind _asbp_star_projectile (Utilities|Casting|CastToBP_StarProjectile OtherActor)
        (:then
          (Utilities|Casting|CastToBP_Star (Game|GetInstigator _asbp_star_projectile))
          (Variables|Default|SetImmuneToProjectile false)
          (Utilities|FlowControl|Delay 0.5)
          (Variables|Default|SetImmuneToProjectile true))
        (:CastFailed
          (bind _asshape (Utilities|Casting|CastToShape OtherActor))
          (if (Variables|Default|GetFacingRight)
            (Character|LaunchCharacter _asshape "400.000000,0.000000,200.000000" false false)
            (elif (Variables|Default|GetFacingLeft)
              (Character|LaunchCharacter _asshape "-400.000000,0.000000,200.000000" false false))))))))

(event Custom|Turn
  ;[1 1 1] Turn
  (if (Variables|Default|GetFacingRight)
    (Variables|Default|SetFacingRight false)
    (Variables|Default|SetFacingLeft true)
    (Transformation|SetActorRotation "0.000000,180.000000,0.000000")
    (else
      (Variables|Default|SetFacingRight true)
      (Variables|Default|SetFacingLeft false)
      (Transformation|SetActorRotation "0, 0, 0"))))

(event EventPlayDamageAnimation
  ;[1 1 1] Damage Event
  (if true
    (Variables|Default|SetInDamageCoolDown true)
    (Sprite|SetFlipbook (Variables|Default|GetSprite) "/Game/Import_Assets/Sprites/EnemySquare/Sprites/Animations/EnemySquare_Hit.EnemySquare_Hit")
    (Variables|/Script/Engine.CharacterMovementComponent|SetMaxWalkSpeed (Variables|Character|GetCharacterMovement) 0.0)
    (Utilities|FlowControl|Delay 0.5)
    (Variables|/Script/Engine.CharacterMovementComponent|SetMaxWalkSpeed (Variables|Character|GetCharacterMovement) 6e+02)
    (Variables|Default|SetWalking false)
    (Variables|Default|SetInDamageCoolDown false)
    (Sprite|SetFlipbook (Variables|Default|GetSprite) "/Game/Import_Assets/Sprites/EnemySquare/Sprites/Animations/EnemySquare_Idle.EnemySquare_Idle")))

(event EventAttack
  ;[1 1 1] Square attack
  (if (not (Variables|Default|GetCoolDownActive))
    (Variables|Default|SetInAttackAnimation true)
    (Sprite|SetFlipbook (Variables|Default|GetSprite) "/Game/Import_Assets/Sprites/EnemySquare/Sprites/Animations/EnemySquare_Mirror.EnemySquare_Mirror")
    (Variables|/Script/Engine.CharacterMovementComponent|SetMaxWalkSpeed (Variables|Character|GetCharacterMovement) 0.0)
    (Utilities|FlowControl|Delay 1.0)
    (Variables|/Script/Engine.CharacterMovementComponent|SetMaxWalkSpeed (Variables|Character|GetCharacterMovement) 6e+02)
    (Sprite|SetFlipbook (Variables|Default|GetSprite) "/Game/Import_Assets/Sprites/EnemySquare/Sprites/Animations/EnemySquare_Idle.EnemySquare_Idle")
    (Variables|Default|SetInAttackAnimation false)
    (Variables|Default|SetWalking false)))

(event EventTick
  (params (DeltaSeconds :type Float%20%28single-precision%29))
  ;[1 1 1] Sets to walking state
  (if (not (and (AI|Components|NavMovement|IsFalling (Variables|Character|GetCharacterMovement)) (Variables|Default|GetInAttackAnimation)))
    (if (not (Variables|Default|GetWalking))
      (Variables|Default|SetWalking true)
      (Sprite|SetFlipbook (Variables|Default|GetSprite) "/Game/Import_Assets/Sprites/EnemySquare/Sprites/Animations/EnemySquare_Move.EnemySquare_Move"))))

(fn ConstructionScript
  (|CallParentFunction))