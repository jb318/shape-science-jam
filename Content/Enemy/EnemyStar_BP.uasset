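; Paper2D star enemy that patrols by constantly walking forward, rotating 180 degrees when its wall detector overlaps something.
; Pawn sensing runs an attack-range check, though TargetPlayer is set to None just before the distance is measured.
; In range, it stops, spawns a projectile at the muzzle and plays the attack flipbook, gated by a DoOnce reset after a delay.
; Beyond range, it restores walk speed and the moving flipbook.
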(event OnComponentBeginOverlap(WallDetector)
  (params (OverlappedComponent :type Primitive%20Component%20Object%20Reference) (OtherActor :type Actor%20Object%20Reference) (OtherComp :type Primitive%20Component%20Object%20Reference) (OtherBodyIndex :type Integer) (bFromSweep :type Boolean) (SweepResult :type Hit%20Result%20Structure%20%28by%20ref%29))
  (CallFunction|TurnChar))

(event OnSeePawn(PawnSensingComp)
  (params (Pawn :type Pawn%20Object%20Reference))
  (Variables|Default|SetTargetPlayer 0)
  (if (<= (Transformation|GetDistanceTo Pawn (Variables|Default|GetTargetPlayer)) (Variables|Default|GetAttackRange))
    (Variables|Default|SetbIsAttacking true)
    (Utilities|FlowControl|DoOnce false
      (:Completed
        (CallFunction|PlayAttack)))
    (elif (>= (Transformation|GetDistanceTo Pawn (Variables|Default|GetTargetPlayer)) (Variables|Default|GetAttackRange))
      (Variables|/Script/Engine.CharacterMovementComponent|SetMaxWalkSpeed (Variables|Character|GetCharacterMovement) 2e+02)
      (Variables|Default|SetbIsAttacking false)
      (Sprite|SetFlipbook (Variables|Default|GetPaperFlipbook) (Variables|Default|GetMoving)))))

(event Custom|PlayAttack
  (Variables|/Script/Engine.CharacterMovementComponent|SetMaxWalkSpeed (Variables|Character|GetCharacterMovement) 0.0)
  (Game|SpawnActorfromClass (Variables|Default|GetProjectile) (Transformation|GetWorldTransform (Variables|Default|GetMuzzlePoint)) "Undefined" "MultiplyWithRoot" 0 0)
  (Sprite|SetFlipbook (Variables|Default|GetPaperFlipbook) (Variables|Default|GetAttack))
  (Audio|Components|Audio|Play (Variables|Default|GetPaperFlipbook))
  (Utilities|FlowControl|Delay 2.0)
  (Utilities|FlowControl|DoOnce false) ; enters at Reset
)

(event EventBeginPlay)

(event Collision|EventActorBeginOverlap
  (params (OtherActor :type Actor%20Object%20Reference)))

(event EventTick
  (params (DeltaSeconds :type Float%20%28single-precision%29))
  (Pawn|Input|AddMovementInput (Transformation|GetActorForwardVector) 1.0 false)
  (if (and (not (Variables|Default|GetbIsAttacking)) (> (Math|Vector|VectorLength (Transformation|GetVelocity)) 0.0))
    (Sprite|SetFlipbook (Variables|Default|GetPaperFlipbook) (Variables|Default|GetMoving))))

(fn ConstructionScript)

(fn TurnChar
  (Transformation|SetActorRotation (Math|Rotator|CombineRotators (Transformation|GetActorRotation) "0.000000,180.000000,0.000000")))