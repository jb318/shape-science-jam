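; Circle enemy Blueprint, a rolling flipbook character that reverses direction at walls and ledges.
; Wall overlap begin and ledge overlap end both call Turn, which flips the facing flags and rotates the actor.
; Attack, when grounded, halts movement for a brief dash animation while CanHitEnemy is set.
; Damage, unless ImmuneToProjectile, pauses movement for a hit animation, then clears Walking so Tick can restore the rolling flipbook.
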(event OnComponentBeginOverlap(WallDetector)
  (params (OverlappedComponent :type Primitive%20Component%20Object%20Reference) (OtherActor :type Actor%20Object%20Reference) (OtherComp :type Primitive%20Component%20Object%20Reference) (OtherBodyIndex :type Integer) (bFromSweep :type Boolean) (SweepResult :type Hit%20Result%20Structure%20%28by%20ref%29))
  ;[1 1 1] Wall and Ledge detection
  (CallFunction|Turn))

(event OnComponentEndOverlap(LedgeDetector)
  (params (OverlappedComponent :type Primitive%20Component%20Object%20Reference) (OtherActor :type Actor%20Object%20Reference) (OtherComp :type Primitive%20Component%20Object%20Reference) (OtherBodyIndex :type Integer))
  ;[1 1 1] Wall and Ledge detection
  (CallFunction|Turn))

(event Custom|Turn
  ;[1 1 1] Wall and Ledge detection
  (if (Variables|Default|GetFacingRight)
    (Variables|Default|SetFacingRight false)
    (Variables|Default|SetFacingLeft true)
    (Transformation|SetActorRotation "0.000000,180.000000,0.000000")
    (else
      (Variables|Default|SetFacingRight true)
      (Variables|Default|SetFacingLeft false)
      (Transformation|SetActorRotation "0, 0, 0"))))

(event EventAttack
  ;[1 1 1] Circle Attack
  (if (not (AI|Components|NavMovement|IsFalling (Variables|Character|GetCharacterMovement)))
    (Variables|Default|SetInAttackAnimation true)
    (Variables|Default|SetCanHitEnemy true)
    (Sprite|SetFlipbook (Variables|Default|GetSprite) "/Game/Import_Assets/Sprites/EnemyCircles/Animations/EnemyCircle_Dash.EnemyCircle_Dash")
    (Variables|/Script/Engine.CharacterMovementComponent|SetMaxWalkSpeed (Variables|Character|GetCharacterMovement) 0.0)
    (Utilities|FlowControl|Delay 0.2)
    (Variables|/Script/Engine.CharacterMovementComponent|SetMaxWalkSpeed (Variables|Character|GetCharacterMovement) 6e+02)
    (Sprite|SetFlipbook (Variables|Default|GetSprite) "/Game/Import_Assets/Sprites/EnemyCircles/Animations/EnemyCircle_Idle.EnemyCircle_Idle")
    (Variables|Default|SetCanHitEnemy false)))

(event EventTick
  (params (DeltaSeconds :type Float%20%28single-precision%29))
  ;[1 1 1] Walk animation
  (if (not (and (AI|Components|NavMovement|IsFalling (Variables|Character|GetCharacterMovement)) (Variables|Default|GetInAttackAnimation)))
    (if (not (Variables|Default|GetWalking))
      (Variables|Default|SetWalking true)
      (Sprite|SetFlipbook (Variables|Default|GetSprite) "/Game/Import_Assets/Sprites/EnemyCircles/Animations/EnemyCircle_Rolling.EnemyCircle_Rolling"))))

(event EventPlayDamageAnimation
  ;[1 1 1] Damage animations
  (if (not (Variables|Default|GetImmuneToProjectile))
    (Variables|Default|SetInDamageCoolDown true)
    (Sprite|SetFlipbook (Variables|Default|GetSprite) "/Game/Import_Assets/Sprites/EnemyCircles/Animations/EnemyCircle_Hit.EnemyCircle_Hit")
    (Variables|/Script/Engine.CharacterMovementComponent|SetMaxWalkSpeed (Variables|Character|GetCharacterMovement) 0.0)
    (Utilities|FlowControl|Delay 0.5)
    (Variables|/Script/Engine.CharacterMovementComponent|SetMaxWalkSpeed (Variables|Character|GetCharacterMovement) 6e+02)
    (Variables|Default|SetWalking false)
    (Variables|Default|SetInDamageCoolDown false)
    (Sprite|SetFlipbook (Variables|Default|GetSprite) "/Game/Import_Assets/Sprites/EnemyCircles/Animations/EnemyCircle_Idle.EnemyCircle_Idle")))

(fn ConstructionScript
  (|CallParentFunction))