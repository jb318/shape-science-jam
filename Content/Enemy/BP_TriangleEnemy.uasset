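; Triangle enemy Blueprint that handles the enemy's flipbook animations, turning, attack and damage reactions, and applies the triangle flipbook to its two projectiles after spawn.
; Wall detector overlaps and ledge detector overlap ends trigger a turn, which flips the actor's rotation and plays a rotate animation.
; Attack and damage events briefly halt movement through walk speed and delays, then clear the Walking flag so Tick can restore the walk flipbook.
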(event OnComponentBeginOverlap(WallDetector)
  (params (OverlappedComponent :type Primitive%20Component%20Object%20Reference) (OtherActor :type Actor%20Object%20Reference) (OtherComp :type Primitive%20Component%20Object%20Reference) (OtherBodyIndex :type Integer) (bFromSweep :type Boolean) (SweepResult :type Hit%20Result%20Structure%20%28by%20ref%29))
  ;[1 1 1] Turns AI
  (CallFunction|Turn))

(event OnComponentEndOverlap(LedgeDetector)
  (params (OverlappedComponent :type Primitive%20Component%20Object%20Reference) (OtherActor :type Actor%20Object%20Reference) (OtherComp :type Primitive%20Component%20Object%20Reference) (OtherBodyIndex :type Integer))
  ;[1 1 1] Turns AI
  (CallFunction|Turn))

(event Custom|Turn
  ;[1 1 1] Turns AI
  (if (Variables|Default|GetFacingRight)
    (Variables|Default|SetFacingRight false)
    (Variables|Default|SetFacingLeft true)
    (Transformation|SetActorRotation "0.000000,180.000000,0.000000")
    (Variables|Default|SetRotating true)
    (Sprite|SetFlipbook (Variables|Default|GetSprite) "/Game/Import_Assets/Sprites/EnemyTriangle/Animations/EnemyTriangle_Rotate.EnemyTriangle_Rotate")
    (Utilities|FlowControl|Delay 0.333)
    (Variables|Default|SetRotating false)
    (Variables|Default|SetWalking false)
    (else
      (Variables|Default|SetFacingRight true)
      (Variables|Default|SetFacingLeft false)
      (Transformation|SetActorRotation "0, 0, 0")
      (Variables|Default|SetRotating true)
      (Sprite|SetFlipbook (Variables|Default|GetSprite) "/Game/Import_Assets/Sprites/EnemyTriangle/Animations/EnemyTriangle_Rotate.EnemyTriangle_Rotate")
      (Utilities|FlowControl|Delay 0.333)
      (Variables|Default|SetRotating false)
      (Variables|Default|SetWalking false))))

(event EventAttack
  ;[1 1 1] Triangle attack
  (if (not (AI|Components|NavMovement|IsFalling (Variables|Character|GetCharacterMovement)))
    (Variables|Default|SetInAttackAnimation true)
    (Sprite|SetFlipbook (Variables|Default|GetSprite) "/Game/Import_Assets/Sprites/EnemyTriangle/Animations/EnemyTriagnle_Attack.EnemyTriagnle_Attack")
    (Variables|/Script/Engine.CharacterMovementComponent|SetMaxWalkSpeed (Variables|Character|GetCharacterMovement) 0.0)
    (Utilities|FlowControl|Delay 0.25)
    (Variables|/Script/Engine.CharacterMovementComponent|SetMaxWalkSpeed (Variables|Character|GetCharacterMovement) 6e+02)
    (Sprite|SetFlipbook (Variables|Default|GetSprite) "/Game/Import_Assets/Sprites/EnemyTriangle/Animations/EnemyTriagnle_Attack.EnemyTriagnle_Attack")
    (Variables|Default|SetInAttackAnimation false)
    (Variables|Default|SetWalking false)
    (Variables|Default|SetCoolDownActive false)))

(event EventBeginPlay
  (bind _projectile2 (Variables|Default|GetProjectile2))
  (bind _projectile1 (Variables|Default|GetProjectile1))
  ;[1 1 1] Sets the flipbook of triangle projectiles
  (Utilities|FlowControl|Delay 0.2)
  (Utilities|IsValid _projectile1
    (:Is%20Valid
      (Sprite|SetFlipbook (Variables|/Script/shape_science_jam.Projectile|GetFlipbook _projectile1) "/Game/Import_Assets/Sprites/EnemyTriangle/Animations/EnemyTriangle_RightIdle.EnemyTriangle_RightIdle")
      (Utilities|IsValid _projectile2
        (:Is%20Valid
          (Sprite|SetFlipbook (Variables|/Script/shape_science_jam.Projectile|GetFlipbook _projectile2) "/Game/Import_Assets/Sprites/EnemyTriangle/Animations/EnemyTriangle_RightIdle.EnemyTriangle_RightIdle"))))))

(event EventTick
  (params (DeltaSeconds :type Float%20%28single-precision%29))
  ;[1 1 1] Walk animation
  (if (not (Math|Boolean|ANDBoolean (AI|Components|NavMovement|IsFalling (Variables|Character|GetCharacterMovement)) (Variables|Default|GetInAttackAnimation) (Variables|Default|GetRotating)))
    (if (not (Variables|Default|GetWalking))
      (Variables|Default|SetWalking true)
      (Sprite|SetFlipbook (Variables|Default|GetSprite) "/Game/Import_Assets/Sprites/EnemyTriangle/Animations/EnemyTriangle_RightIdle.EnemyTriangle_RightIdle"))))

(event EventPlayDamageAnimation
  ;[1 1 1] Damage animations
  (if (not (Variables|Default|GetImmuneToProjectile))
    (Variables|Default|SetInDamageCoolDown true)
    (Sprite|SetFlipbook (Variables|Default|GetSprite) "/Game/Import_Assets/Sprites/EnemyTriangle/Animations/EnemyTriangle_Hit.EnemyTriangle_Hit")
    (Variables|/Script/Engine.CharacterMovementComponent|SetMaxWalkSpeed (Variables|Character|GetCharacterMovement) 0.0)
    (Utilities|FlowControl|Delay 0.5)
    (Variables|/Script/Engine.CharacterMovementComponent|SetMaxWalkSpeed (Variables|Character|GetCharacterMovement) 6e+02)
    (Variables|Default|SetWalking false)
    (Variables|Default|SetInDamageCoolDown false)
    (Sprite|SetFlipbook (Variables|Default|GetSprite) "/Game/Import_Assets/Sprites/EnemyTriangle/Animations/EnemyTriangle_RightIdle.EnemyTriangle_RightIdle")))

(fn ConstructionScript
  (|CallParentFunction))