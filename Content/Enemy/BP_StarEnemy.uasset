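; Star enemy Blueprint that gives its three projectiles the star flipbook shortly after BeginPlay and plays a walk animation.
; It turns around by flipping actor rotation when its wall detector begins an overlap or its ledge detector ends one.
; Tick sets the walk flipbook whenever Walking is false, as its falling check is effectively disabled.
; Attack and damage events do nothing; their timed animation and movement-pause chains are disconnected.
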(event OnComponentBeginOverlap(WallDetector)
  (params (OverlappedComponent :type Primitive%20Component%20Object%20Reference) (OtherActor :type Actor%20Object%20Reference) (OtherComp :type Primitive%20Component%20Object%20Reference) (OtherBodyIndex :type Integer) (bFromSweep :type Boolean) (SweepResult :type Hit%20Result%20Structure%20%28by%20ref%29))
  ;[1 1 1] Turns AI
  (CallFunction|Turn))

(event OnComponentEndOverlap(LedgeDetector)
  (params (OverlappedComponent :type Primitive%20Component%20Object%20Reference) (OtherActor :type Actor%20Object%20Reference) (OtherComp :type Primitive%20Component%20Object%20Reference) (OtherBodyIndex :type Integer))
  ;[1 1 1] Turns AI
  (CallFunction|Turn))

(event Custom|Turn
  ;[1 1 1] Turns AI
  (if (Variables|Default|GetFacingRight)
    (Variables|Default|SetFacingRight false)
    (Variables|Default|SetFacingLeft true)
    (Transformation|SetActorRotation "0.000000,180.000000,0.000000")
    (else
      (Variables|Default|SetFacingRight true)
      (Variables|Default|SetFacingLeft false)
      (Transformation|SetActorRotation "0, 0, 0"))))

(event EventAttack
  ;[1 1 1] Star attack
  (if (not (AI|Components|NavMovement|IsFalling (Variables|Character|GetCharacterMovement)))
    _))

(event EventBeginPlay
  (bind _projectile2 (Variables|Default|GetProjectile2))
  (bind _projectile3 (Variables|Default|GetProjectile3))
  (bind _projectile1 (Variables|Default|GetProjectile1))
  ;[1 1 1] Sets the flipbook of star projectiles
  (Utilities|FlowControl|Delay 0.2)
  (Utilities|IsValid _projectile1
    (:Is%20Valid
      (Sprite|SetFlipbook (Variables|/Script/shape_science_jam.Projectile|GetFlipbook _projectile1) "/Game/Import_Assets/Sprites/EnemyStar/Animations/EnemyStar_Projectile.EnemyStar_Projectile")
      (Utilities|IsValid _projectile2
        (:Is%20Valid
          (Sprite|SetFlipbook (Variables|/Script/shape_science_jam.Projectile|GetFlipbook _projectile2) "/Game/Import_Assets/Sprites/EnemyStar/Animations/EnemyStar_Projectile.EnemyStar_Projectile")
          (Utilities|IsValid _projectile3
            (:Is%20Valid
              (Sprite|SetFlipbook (Variables|/Script/shape_science_jam.Projectile|GetFlipbook _projectile3) "/Game/Import_Assets/Sprites/EnemyStar/Animations/EnemyStar_Projectile.EnemyStar_Projectile"))))))))

(event EventTick
  (params (DeltaSeconds :type Float%20%28single-precision%29))
  ;[1 1 1] Walk animation
  (if (not (and (AI|Components|NavMovement|IsFalling (Variables|Character|GetCharacterMovement)) false))
    (if (not (Variables|Default|GetWalking))
      (Variables|Default|SetWalking true)
      (Sprite|SetFlipbook (Variables|Default|GetSprite) "/Game/Import_Assets/Sprites/EnemyStar/Animations/EnemyStar_Walk.EnemyStar_Walk"))))

(event EventPlayDamageAnimation
  ;[1 1 1] Damage animations
  (if (not (Variables|Default|GetImmuneToProjectile))
    _))

(fn ConstructionScript
  (|CallParentFunction))