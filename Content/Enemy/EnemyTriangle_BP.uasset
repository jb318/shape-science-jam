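; Paper2D enemy that walks forward, turns around on wall-detector overlap and fires projectiles when pawn sensing triggers an attack.
; Tick drives movement and the moving flipbook until IsAttacking is set.
; A sighting passing the range check, measured against a just-cleared TargetPawn, enters a DoOnce that stops movement, spawns a projectile and re-arms after a delay.
; Nothing here restores walk speed or clears IsAttacking.
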(event OnSeePawn(PawnSensingComp)
  (params (Pawn :type Pawn%20Object%20Reference))
  (Variables|Default|SetTargetPawn 0)
  (if (<= (Transformation|GetDistanceTo Pawn (Variables|Default|GetTargetPawn)) (Variables|Default|GetAttackRange))
    (Variables|Default|SetbIsAttacking true)
    (Utilities|FlowControl|DoOnce false
      (:Completed
        (CallFunction|PlayAttack)))))

(event OnComponentBeginOverlap(WallDetector)
  (params (OverlappedComponent :type Primitive%20Component%20Object%20Reference) (OtherActor :type Actor%20Object%20Reference) (OtherComp :type Primitive%20Component%20Object%20Reference) (OtherBodyIndex :type Integer) (bFromSweep :type Boolean) (SweepResult :type Hit%20Result%20Structure%20%28by%20ref%29))
  (CallFunction|TurnChar))

(event Custom|PlayAttack
  (bind _paperflipbook (Variables|Default|GetPaperFlipbook))
  (Variables|/Script/Engine.CharacterMovementComponent|SetMaxWalkSpeed (Variables|Character|GetCharacterMovement) 0.0)
  (Game|SpawnActorfromClass (Variables|Default|GetProjectile) (Transformation|GetWorldTransform (Variables|Default|GetMuzzlePoint)) "Undefined" "MultiplyWithRoot" 0 0)
  (Sprite|SetFlipbook _paperflipbook (Variables|Default|GetAttack))
  (Audio|Components|Audio|Play _paperflipbook)
  (Utilities|FlowControl|Delay 2.0)
  (Utilities|FlowControl|DoOnce false) ; enters at Reset
)

(event EventBeginPlay)

(event EventTick
  (params (DeltaSeconds :type Float%20%28single-precision%29))
  (Pawn|Input|AddMovementInput (Transformation|GetActorForwardVector) 1.0 false)
  (if (and (not (Variables|Default|GetbIsAttacking)) (> (Math|Vector|VectorLength (Transformation|GetVelocity)) 0.0))
    (Sprite|SetFlipbook (Variables|Default|GetPaperFlipbook) (Variables|Default|GetMoving))))

(fn ConstructionScript)

(fn TurnChar
  (Transformation|SetActorRotation (Math|Rotator|CombineRotators (Transformation|GetActorRotation) "0.000000,180.000000,0.000000")))